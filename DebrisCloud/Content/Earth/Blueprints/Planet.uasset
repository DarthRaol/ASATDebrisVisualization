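; Configurable planet actor with optional moon, clouds, atmosphere and night lights, animated as a simple spin and orbit simulation.
; The construction script sets visibility, dynamic material instances, tilts, scales and helper orbit and axis graphics from variables.
; Tick accumulates a shared time value that drives planet spin, cloud rotation and moon orbit, each reversible.
; Demo keys toggle the graphics and adjust PlanetDayLengthMinutes, which acts as a speed multiplier for spin and orbit.
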(event `self.ReceiveBeginPlay`
  ;[1 1 1] Demo Level Controllers
  (`self.EnableInput` (`GameplayStatics.GetPlayerController` 0)))

(event `Key|SpaceBar`
  (params (Key :type "Key Structure"))
  (bind _planet_axial_tilt_graphic (`self.Planet Axial Tilt Graphic`))
  ;[1 1 1] Demo Level Controllers
  (:`Pressed`
    (`/Engine/EditorBlueprintResources/StandardMacros.FlipFlop`
      (:`A`
        (`SceneComponent.SetVisibility` _planet_axial_tilt_graphic false false)
        (`SceneComponent.SetVisibility` (`self.PlanetOrbitGraphic`) false false)
        (`SceneComponent.SetVisibility` (`self.MoonOrbitGraphic`) false false)
        (`SceneComponent.SetVisibility` (`self.Moon Axial Tilt Graphic`) false false))
      (:`B`
        (`SceneComponent.SetVisibility` _planet_axial_tilt_graphic true false)
        (`SceneComponent.SetVisibility` (`self.PlanetOrbitGraphic`) true false)
        (`SceneComponent.SetVisibility` (`self.MoonOrbitGraphic`) true false)
        (`SceneComponent.SetVisibility` (`self.Moon Axial Tilt Graphic`) true false)))))

(event `Key|Add`
  (params (Key :type "Key Structure"))
  ;[1 1 1] Demo Level Controllers
  (:`Pressed`
    (set `self.Planet Day Length (Minutes)` (+ (`self.Planet Day Length (Minutes)`) 25))))

(event `self.ReceiveTick`
  (params (DeltaSeconds :type "Float (single-precision)"))
  (bind _planet_scale_rotation (`self.Planet Scale/Rotation`))
  (bind _moonorbit (`self.MoonOrbit`))
  (bind _globalspeedupdate (`self.GlobalSpeedUpdate`))
  (bind _clouds (`self.Clouds`))
  (bind _returnvalue (* (`self.Planet Day Length (Minutes)`) (`self.GlobalSpeedUpdate`)))
  (bind _returnvalue_2 (* (`self.CloudsRotation Speed (x)`) _globalspeedupdate))
  (bind _returnvalue_3 (* (`self.CloudsRotation Speed (y)`) _globalspeedupdate))
  (bind _returnvalue_4 (* (`self.CloudsRotation Speed (z)`) _globalspeedupdate))
  (bind _returnvalue_5 (/ _returnvalue (`self.Month Length (Days)`)))
  ;[1 1 1] Global Time Setup
  (set `self.GlobalSpeedUpdate` (+ (* DeltaSeconds -6.0) (`self.GlobalSpeedUpdate`)))
  (`|ExecutionSequence`
    (:`then_0`
      ;[1 1 1] Moon Simulation
      (if (`self.Moon Direction Reversed`)
        (`SceneComponent.K2_SetRelativeRotation` _moonorbit (`KismetMathLibrary.MakeRotator` 0.0 0.0 (* _returnvalue_5 -1.0)) false false)
        (else
          (`SceneComponent.K2_SetRelativeRotation` _moonorbit (`KismetMathLibrary.MakeRotator` 0.0 0.0 _returnvalue_5) false false))))
    (:`then_1`
      ;[1 1 1] Planet Simulation
      (if (`self.Planet Direction Reversed`)
        (`SceneComponent.K2_SetRelativeRotation` _planet_scale_rotation (`KismetMathLibrary.MakeRotator` 0.0 0.0 (* _returnvalue -1.0)) false false)
        (else
          (`SceneComponent.K2_SetRelativeRotation` _planet_scale_rotation (`KismetMathLibrary.MakeRotator` 0.0 0.0 _returnvalue) false false))))
    (:`then_2`
      ;[1 1 1] Clouds Simulation
      (if (`self.Clouds Direction Reversed`)
        (`SceneComponent.K2_SetRelativeRotation` _clouds (`KismetMathLibrary.MakeRotator` (* _returnvalue_2 -0.1) (* _returnvalue_3 -0.1) (* _returnvalue_4 -0.1)) false false)
        (`SceneComponent.K2_SetRelativeRotation` (`self.StandaloneClouds`) (`KismetMathLibrary.MakeRotator` (* _returnvalue_2 -0.1) (* _returnvalue_3 -0.1) (* _returnvalue_4 -0.1)) false false)
        (else
          (`SceneComponent.K2_SetRelativeRotation` _clouds (`KismetMathLibrary.MakeRotator` (* _returnvalue_2 0.1) (* _returnvalue_3 0.1) (* _returnvalue_4 0.1)) false false)
          (`SceneComponent.K2_SetRelativeRotation` (`self.StandaloneClouds`) (`KismetMathLibrary.MakeRotator` (* _returnvalue_2 0.1) (* _returnvalue_3 0.1) (* _returnvalue_4 0.1)) false false))))))

(event `Key|Subtract`
  (params (Key :type "Key Structure"))
  ;[1 1 1] Demo Level Controllers
  (:`Pressed`
    (set `self.Planet Day Length (Minutes)` (- (`self.Planet Day Length (Minutes)`) 25))))

(event `Key|NumPadZero`
  (params (Key :type "Key Structure"))
  ;[1 1 1] Demo Level Controllers
  (:`Pressed`
    (set `self.Planet Day Length (Minutes)` 1)))

(fn `UserConstructionScript`
  (bind _earth (`self.Earth`))
  (bind _clouds (`self.Clouds`))
  (bind _planetscale____ (`self.PlanetScale (%)`))
  (bind _clouds_2 (`self.Clouds`))
  (bind _standaloneclouds (`self.StandaloneClouds`))
  (bind _atmosphere (`self.Atmosphere`))
  (bind _standaloneclouds_2 (`self.StandaloneClouds`))
  (bind _moon (`self.Moon`))
  (bind _moon_2 (`self.Moon`))
  (bind _planet_axial_tilt_graphic (`self.Planet Axial Tilt Graphic`))
  (bind _atmosphere_2 (`self.Atmosphere`))
  (bind _nightlights (`self.NightLights`))
  (bind _nightlights_2 (`self.NightLights`))
  (bind _moon_scale____ (`self.Moon Scale (%)`))
  (bind _returnvalue (/ (`self.Moon Scale (%)`) 366.6670333337))
  (bind _returnvalue_2 (/ _moon_scale____ 653.334291556961))
  (bind _returnvalue_3 (/ (`self.Moon Distance`) 200.0))
  (bind _returnvalue_4 (/ _planetscale____ 200.0))
  (bind _returnvalue_5 (+ (* (`self.Atmosphere Thickness`) 0.001) 1.0))
  (bind _returnvalue_6 (+ (* (`self.Clouds Height`) 0.001) 1.0))
  (bind _returnvalue_7 (+ (* (`self.PlanetScale (%)`) 0.01) 0.0))
  (`|ExecutionSequence`
    (:`then_0`
      ;[1 1 1] Planet Properties
      (`|ExecutionSequence`
        (:`then_0`
          (if (`self.Has Clouds`)
            (if (`self.Standalone Clouds`)
              (`SceneComponent.SetVisibility` _clouds_2 false false)
              (`SceneComponent.SetVisibility` _standaloneclouds true false)
              (else
                (`SceneComponent.SetVisibility` _clouds_2 true false)
                (`SceneComponent.SetVisibility` _standaloneclouds false false)))
            (else
              (`SceneComponent.SetVisibility` (`self.Clouds`) false false)
              (`SceneComponent.SetVisibility` (`self.StandaloneClouds`) false false))))
        (:`then_1`
          (if (`self.Has Atmosphere`)
            (`SceneComponent.SetVisibility` _atmosphere_2 true false)
            (else
              (`SceneComponent.SetVisibility` _atmosphere_2 false false))))
        (:`then_2`
          (if (`self.Has Moon`)
            (`SceneComponent.SetVisibility` _moon true false)
            (else
              (`SceneComponent.SetVisibility` _moon false false))))
        (:`then_3`
          (if (`self.NightLigts`)
            (`SceneComponent.SetVisibility` _nightlights true false)
            (else
              (`SceneComponent.SetVisibility` _nightlights false false))))))
    (:`then_1`
      ;[1 1 1] Dynamic Materials
      (`|ExecutionSequence`
        (:`then_0`
          (bind _returnvalue_8 (`PrimitiveComponent.CreateDynamicMaterialInstance` _earth 0 "/Game/Earth/Materials/Planet_Inst.Planet_Inst" "None"))
          (`MaterialInstanceDynamic.SetTextureParameterValue` _returnvalue_8 "Base Color" (`self.Planet Diffuse`))
          (`MaterialInstanceDynamic.SetTextureParameterValue` _returnvalue_8 "Normal" (`self.Planet Normal`))
          (`MaterialInstanceDynamic.SetTextureParameterValue` _returnvalue_8 "Specular" (`self.Planet Specular`))
          (`MeshComponent.SetScalarParameterValueOnMaterials` _earth "Roughness Intensity" (`self.Roughness Intensity`))
          (`MeshComponent.SetScalarParameterValueOnMaterials` _earth "Specular Intensity" (- (`self.Specular Intensity`) 1.0))
          (`MeshComponent.SetScalarParameterValueOnMaterials` _earth "Normal Intensity" (- (`self.Normal Intensity`) 1.0)))
        (:`then_1`
          (bind _returnvalue_9 (`PrimitiveComponent.CreateDynamicMaterialInstance` _clouds 0 "/Game/Earth/Materials/Clouds_Inst.Clouds_Inst" "None"))
          (`MaterialInstanceDynamic.SetTextureParameterValue` _returnvalue_9 "Clouds Texture" (`self.Clouds Diffuse`))
          (`MaterialInstanceDynamic.SetTextureParameterValue` _returnvalue_9 "CloudsNormal" (`self.Clouds Normal`))
          (`MaterialInstanceDynamic.SetVectorParameterValue` _returnvalue_9 "Clouds Color" (`self.Clouds Color`))
          (`MeshComponent.SetScalarParameterValueOnMaterials` _clouds "CloudsOpacity" (/ (`self.Clouds Opacity (%)`) 100.0))
          (`MeshComponent.SetScalarParameterValueOnMaterials` _clouds "CloudsNormalIntensity" (- (/ (`self.Clouds Normal Intensity (%)`) 100.0) 1.0)))
        (:`then_2`
          (bind _returnvalue_10 (`PrimitiveComponent.CreateDynamicMaterialInstance` _standaloneclouds_2 0 "/Game/Earth/Materials/Clouds_Inst.Clouds_Inst" "None"))
          (`MaterialInstanceDynamic.SetTextureParameterValue` _returnvalue_10 "Clouds Texture" (`self.Clouds Diffuse`))
          (`MaterialInstanceDynamic.SetTextureParameterValue` _returnvalue_10 "CloudsNormal" (`self.Clouds Normal`))
          (`MaterialInstanceDynamic.SetVectorParameterValue` _returnvalue_10 "Clouds Color" (`self.Clouds Color`))
          (`MeshComponent.SetScalarParameterValueOnMaterials` _standaloneclouds_2 "CloudsOpacity" (/ (`self.Clouds Opacity (%)`) 100.0))
          (`MeshComponent.SetScalarParameterValueOnMaterials` _standaloneclouds_2 "CloudsNormalIntensity" (- (/ (`self.Clouds Normal Intensity (%)`) 100.0) 1.0)))
        (:`then_3`
          (bind _returnvalue_11 (`PrimitiveComponent.CreateDynamicMaterialInstance` _atmosphere 0 "/Game/Earth/Materials/Atmosphere_Inst.Atmosphere_Inst" "None"))
          (`MaterialInstanceDynamic.SetVectorParameterValue` _returnvalue_11 "Atmosphere Color" (`self.Atmosphere Color`))
          (`MeshComponent.SetScalarParameterValueOnMaterials` _atmosphere "Atmosphere Opacity" (/ (`self.Atmosphere Opacity (%)`) 33.3)))
        (:`then_4`
          (bind _returnvalue_12 (`PrimitiveComponent.CreateDynamicMaterialInstance` _moon_2 0 "/Game/Earth/Materials/Moon_Inst.Moon_Inst" "None"))
          (`MaterialInstanceDynamic.SetTextureParameterValue` _returnvalue_12 "Moon Diffuse" (`self.Moon Diffuse`))
          (`MaterialInstanceDynamic.SetTextureParameterValue` _returnvalue_12 "Moon Normal" (`self.Moon Normal`))
          (`MeshComponent.SetScalarParameterValueOnMaterials` _moon_2 "Moon Normal Intensity" (`self.Moon Normal Intensity`)))
        (:`then_5`
          (bind _returnvalue_13 (`PrimitiveComponent.CreateDynamicMaterialInstance` _nightlights_2 0 "/Game/Earth/Materials/Masters/NightLights.NightLights" "None"))
          (`MaterialInstanceDynamic.SetTextureParameterValue` _returnvalue_13 "NightLights" (`self.NightLights Diffuse`))
          (`MeshComponent.SetScalarParameterValueOnMaterials` _nightlights_2 "NightLights Intensity" (/ (`self.NightLights Intensity`) 100.0)))))
    (:`then_2`
      ;[1 1 1] Transform Settings
      (`SceneComponent.K2_SetRelativeRotation` (`self.Axial Tilt`) (`KismetMathLibrary.MakeRotator` (`self.Planet AxialTilt (x)`) (`self.Planet AxialTilt (y)`) (`self.Planet AxialTilt (z)`)) false false)
      (`SceneComponent.SetRelativeScale3D` (`self.Clouds`) (`KismetMathLibrary.MakeVector` _returnvalue_6 _returnvalue_6 _returnvalue_6))
      (`SceneComponent.SetRelativeScale3D` (`self.StandaloneClouds`) (`KismetMathLibrary.MakeVector` _returnvalue_6 _returnvalue_6 _returnvalue_6))
      (`SceneComponent.SetRelativeScale3D` (`self.Atmosphere`) (`KismetMathLibrary.MakeVector` _returnvalue_5 _returnvalue_5 _returnvalue_5))
      (`SceneComponent.K2_SetRelativeLocationAndRotation` (`self.Moon Axial Tilt`) (`KismetMathLibrary.MakeVector` 0.0 (`self.Moon Distance`)) (`KismetMathLibrary.MakeRotator` (`self.Moon Axial Tilt (x)`) (`self.Moon Axial Tilt (y)`) (`self.Moon Axial Tilt (z)`)) false false)
      (`SceneComponent.K2_SetRelativeLocationAndRotation` (`self.Moon`) (0.0 0.0 0.0) (`KismetMathLibrary.MakeRotator` (`self.Moon Rotation (x)`) (`self.Moon Rotation (y)`) (`self.Moon Rotation (z)`)) false false)
      (`SceneComponent.K2_SetRelativeRotation` (`self.MoonOrbitRotation`) (`KismetMathLibrary.MakeRotator` (`self.Moon Orbit (x)`) (`self.Moon Orbit (y)`) (`self.Moon Orbit (z)`)) false false)
      (`SceneComponent.SetRelativeScale3D` (`self.Planet Scale/Rotation`) (`KismetMathLibrary.MakeVector` _returnvalue_7 _returnvalue_7 _returnvalue_7))
      (`SceneComponent.K2_SetRelativeRotation` (`self.Earth`) (`KismetMathLibrary.MakeRotator` (`self.Planet Rotation (x)`) (`self.Planet Rotation (y)`) (`self.Planet Rotation (z)`)) false false)
      (`SceneComponent.SetRelativeScale3D` (`self.Moon`) (`KismetMathLibrary.MakeVector` _returnvalue _returnvalue _returnvalue)))
    (:`then_3`
      ;[1 1 1] Show Graphics
      (`|ExecutionSequence`
        (:`then_0`
          (if (`self.Show Graphics (Recommended)`)
            (`SceneComponent.SetVisibility` _planet_axial_tilt_graphic true false)
            (`SceneComponent.SetVisibility` (`self.PlanetOrbitGraphic`) true false)
            (if (`self.Has Moon`)
              (`SceneComponent.SetVisibility` (`self.MoonOrbitGraphic`) true false)
              (`SceneComponent.SetVisibility` (`self.Moon Axial Tilt Graphic`) true false)
              (else
                (`SceneComponent.SetVisibility` (`self.Moon Axial Tilt Graphic`) true false)
                (`SceneComponent.SetVisibility` (`self.MoonOrbitGraphic`) true false)))
            (else
              (`SceneComponent.SetVisibility` _planet_axial_tilt_graphic false false)
              (`SceneComponent.SetVisibility` (`self.PlanetOrbitGraphic`) false false)
              (`SceneComponent.SetVisibility` (`self.MoonOrbitGraphic`) false false)
              (`SceneComponent.SetVisibility` (`self.Moon Axial Tilt Graphic`) false false))))
        (:`then_1`
          (`SceneComponent.SetRelativeScale3D` (`self.MoonOrbitGraphic`) (`KismetMathLibrary.MakeVector` _returnvalue_3 _returnvalue_3 _returnvalue_3))
          (`SceneComponent.SetRelativeScale3D` (`self.PlanetOrbitGraphic`) (`KismetMathLibrary.MakeVector` _returnvalue_3 _returnvalue_3 _returnvalue_3))
          (`SceneComponent.SetRelativeScale3D` (`self.Planet Axial Tilt Graphic`) (`KismetMathLibrary.MakeVector` _returnvalue_4 _returnvalue_4 (/ _planetscale____ 2.0)))
          (`SceneComponent.SetRelativeScale3D` (`self.Moon Axial Tilt Graphic`) (`KismetMathLibrary.MakeVector` _returnvalue_2 _returnvalue_2 (/ _moon_scale____ 7.333343355569253))))))))