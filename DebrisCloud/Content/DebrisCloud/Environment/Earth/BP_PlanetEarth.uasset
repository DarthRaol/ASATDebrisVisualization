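; Planet Earth actor for the environment, with an Earth body and a night lights layer shaded according to the sun's position.
; The construction script creates dynamic material instances for both components.
; BeginPlay scales the actor from EarthRadius and sets its location.
; Every tick it passes SunPosition to both materials as their LightDirection parameter, so lighting is driven through the shaders.
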(event `self.ReceiveBeginPlay`
  (`self.SetActorScale3D` (* (`self.Earth Radius`) (0.02 0.02 0.02)))
  (`self.K2_SetActorLocation` (0.0 0.0 0.0)))

(event `self.ReceiveTick`
  (params (DeltaSeconds :type "Float (single-precision)"))
  (bind _returnvalue (`KismetMathLibrary.Conv_VectorToLinearColor` (`self.SunPosition`)))
  (bind _dight_light_dim (`self.Dight light DIM`)
    (:`then`
      (`MaterialInstanceDynamic.SetVectorParameterValue` _dight_light_dim "LightDirection" _returnvalue))
    (:`else`
      _))
  (bind _earthdim (`self.EarthDIM`)
    (:`then`
      (`MaterialInstanceDynamic.SetVectorParameterValue` _earthdim "LightDirection" _returnvalue))
    (:`else`)))

(fn `UserConstructionScript`
  (bind _returnvalue (`PrimitiveComponent.CreateDynamicMaterialInstance` (`self.NightLights`) 0 "/Game/Earth/Materials/NightLights_Inst.NightLights_Inst" "None"))
  (set `self.Dight light DIM` _returnvalue)
  (bind _returnvalue_2 (`PrimitiveComponent.CreateDynamicMaterialInstance` (`self.Earth`) 0 "/Game/Earth/Materials/Masters/Planet_Inst.Planet_Inst" "None"))
  (set `self.EarthDIM` _returnvalue_2))