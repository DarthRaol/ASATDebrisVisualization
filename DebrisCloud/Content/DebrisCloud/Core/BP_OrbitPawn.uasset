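; BP_OrbitPawn is a pawn in DebrisCloud that relays camera input to a Satellite reference.
; While ZoomMode is on and Satellite is valid, it forwards the zoom, yaw and pitch axis values to that object's camera handlers.
; The pawn has no camera logic of its own in its graphs, and its HUD widget creation is left unconnected, so it never runs.
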(event `self.ReceiveBeginPlay`)

(event `InputAxis|CameraZoom` :overrideparent false
  (params (AxisValue :type "Float (single-precision)"))
  (if (`self.Zoom mode`)
    (bind _satellite (`self.satellite`)
      (:`then`
        (`SatteliteDebris.OnCameraZoomInput` _satellite AxisValue))
      (:`else`))))

(event `InputAxis|CameraYaw` :overrideparent false
  (params (AxisValue :type "Float (single-precision)"))
  (if (`self.Zoom mode`)
    (bind _satellite (`self.satellite`)
      (:`then`
        (`SatteliteDebris.OnCameraYawAxis` _satellite AxisValue))
      (:`else`))))

(event `InputAxis|CameraPitch` :overrideparent false
  (params (AxisValue :type "Float (single-precision)"))
  (if (`self.Zoom mode`)
    (bind _satellite (`self.satellite`)
      (:`then`
        (`SatteliteDebris.OnCameraPitchAxis` _satellite AxisValue))
      (:`else`))))

(fn `UserConstructionScript`)